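; Tunnel segment for an endless tunnel game, with a spinning wall that RandomizeWall gives one of four hole meshes and a random roll.
; Passing the trigger zone adds score, randomly spawns health packs or enemies ahead, then has TunnelSpawner spawn another tunnel and destroys this one.
; Hitting the wall costs the player health, shows the hurt widget and displays restart on death.
; Score drops on a hit only when it is below one.
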(event OnComponentBeginOverlap(TriggerZone)
  (params (OverlappedComponent :type Primitive%20Component%20Object%20Reference) (OtherActor :type Actor%20Object%20Reference) (OtherComp :type Primitive%20Component%20Object%20Reference) (OtherBodyIndex :type Integer) (bFromSweep :type Boolean) (SweepResult :type Hit%20Result%20Structure%20%28by%20ref%29))
  (bind _returnvalue (Math|Random|RandomFloatinRange -1e+02 2e+02))
  (bind _asbp_player (Utilities|Casting|CastToBP_Player OtherActor))
  (Utilities|FlowControl|Sequence
    (:then_0
      (Variables|/Game/InfiniteMatrix/Blueprints/BP_Player.BP_Player_C|SetScore _asbp_player (+ (Variables|/Game/InfiniteMatrix/Blueprints/BP_Player.BP_Player_C|GetScore _asbp_player) 1.0)))
    (:then_1
      (if (== (Math|Random|RandomIntegerinRange 0 9) 4)
        (Game|SpawnActorfromClass "/Game/InfiniteMatrix/Blueprints/BP_HealthPack_2.BP_HealthPack_2_C" (Math|Transform|MakeTransform (+ (Transformation|GetWorldLocation (Variables|Components|GetTriggerZone)) (Math|Vector|MakeVector (Math|Random|RandomFloatinRange 5e+02 2e+03) (Math|Random|RandomFloatinRange -1e+02 2e+02) (Math|Random|RandomFloatinRange -2e+02 2e+02))) "0, 0, 0" "1,1,1") "Undefined" 0 0)))
    (:then_2
      (if (== (Math|Random|RandomIntegerinRange 0 5) 4)
        (Game|SpawnActorfromClass "/Game/InfiniteMatrix/Blueprints/BP_Enemy.BP_Enemy_C" (Math|Transform|MakeTransform (+ (Transformation|GetWorldLocation (Variables|Components|GetTriggerZone)) (Math|Vector|MakeVector (Math|Random|RandomFloatinRange 5e+02 2e+03) _returnvalue _returnvalue)) "0, 0, 0" "1,1,1") "Undefined" 0 0)))
    (:then_3
      (Default|SpawnTunnelatSpawnPoint (Variables|Default|GetTunnelSpawner))
      (Actor|DestroyActor))))

(event OnComponentBeginOverlap(WallMesh)
  (params (OverlappedComponent :type Primitive%20Component%20Object%20Reference) (OtherActor :type Actor%20Object%20Reference) (OtherComp :type Primitive%20Component%20Object%20Reference) (OtherBodyIndex :type Integer) (bFromSweep :type Boolean) (SweepResult :type Hit%20Result%20Structure%20%28by%20ref%29))
  (Utilities|FlowControl|Sequence
    (:then_0
      (bind _asbp_player (Utilities|Casting|CastToBP_Player OtherActor))
      (Utilities|FlowControl|Sequence
        (:then_1
          (if (< (- (Variables|/Game/InfiniteMatrix/Blueprints/BP_Player.BP_Player_C|GetScore _asbp_player) 1.0) 0.0)
            (Variables|/Game/InfiniteMatrix/Blueprints/BP_Player.BP_Player_C|SetScore _asbp_player (- (Variables|/Game/InfiniteMatrix/Blueprints/BP_Player.BP_Player_C|GetScore _asbp_player) 1.0))))
        (:then_2
          (Variables|/Game/InfiniteMatrix/Blueprints/BP_Player.BP_Player_C|SethasCollided _asbp_player true))
        (:then_3
          (bind _returnvalue (UserInterface|CreateWidget "/Game/InfiniteMatrix/UI/WBP_Hurt.WBP_Hurt_C"))
          (UserInterface|Viewport|AddtoViewport _returnvalue 0))
        (:then_4
          (bind _output_get (Variables|/Game/InfiniteMatrix/Blueprints/BP_Player.BP_Player_C|SetHealth _asbp_player (- (Variables|/Game/InfiniteMatrix/Blueprints/BP_Player.BP_Player_C|GetHealth _asbp_player) 1.0)))
          (Utilities|FlowControl|Sequence
            (:then_0
              (bind _output_get_2 (Variables|/Game/InfiniteMatrix/Blueprints/BP_Player.BP_Player_C|SetIsDead _asbp_player (<= _output_get 0.0)))
              (if _output_get_2
                (Default|DisplayRestart _asbp_player)))
            (:then_1
              (Variables|/Game/InfiniteMatrix/Blueprints/BP_Player.BP_Player_C|SetHealth_percent _asbp_player (/ (Variables|/Game/InfiniteMatrix/Blueprints/BP_Player.BP_Player_C|GetHealth _asbp_player) 4.0)))))))))

(event EventBeginPlay)

(event EventTick
  (params (DeltaSeconds :type Float%20%28single-precision%29))
  (Transformation|AddLocalRotation (Variables|Components|GetWallMesh) (Math|Rotator|MakeRotator (* DeltaSeconds (Variables|Default|GetRotateSpeed)) 0.0 0.0) false false))

(fn ConstructionScript)

(fn RandomizeWall
  (Components|StaticMesh|SetStaticMesh (Variables|Components|GetWallMesh) (Utilities|Select :Index (Math|Random|RandomIntegerinRange 0 3) :Option%200 "/Game/InfiniteMatrix/Meshes/SM_Hole_01.SM_Hole_01" :Option%201 "/Game/InfiniteMatrix/Meshes/SM_Hole_02.SM_Hole_02" :Option%202 "/Game/InfiniteMatrix/Meshes/SM_Hole_03.SM_Hole_03" :Option%203 "/Game/InfiniteMatrix/Meshes/SM_Hole_04.SM_Hole_04"))
  (Transformation|AddLocalRotation (Variables|Components|GetWallMesh) (Math|Rotator|MakeRotator (Math|Random|RandomFloatinRange 0.0 3.6e+02) 0.0 0.0) false false))