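; BP_HPSpawner is a spawner actor that creates BP_HealthPack pickups.
; On BeginPlay it spawns a pack at the player pawn's location, in a short loop that only spawns while NewestHP is invalid.
; Each pack becomes NewestHP, receives a reference to the spawner and runs RandomizeHP.
; SpawnHPAtSpawnPoint chains the next pack from the newest one's SpawnHPPoint, but nothing in this Blueprint's live graphs calls it.
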(event EventBeginPlay
  (CallFunction|SpawnInitialHP))

(event Collision|EventActorBeginOverlap
  (params (OtherActor :type Actor%20Object%20Reference)))

(event EventTick
  (params (DeltaSeconds :type Float%20%28single-precision%29)))

(fn ConstructionScript)

(fn SpawnHP
  (params (SpawnHPLocation :type Vector))
  (bind _returnvalue (Game|SpawnActorfromClass "/Game/InfiniteMatrix/Blueprints/Unneeded/BP_HealthPack.BP_HealthPack_C" (Math|Transform|MakeTransform SpawnHPLocation "0, 0, 0" "1,1,1") "Undefined" 0 0))
  (bind _output_get (Variables|Default|SetNewestHP _returnvalue))
  (Variables|/Game/InfiniteMatrix/Blueprints/Unneeded/BP_HealthPack.BP_HealthPack_C|SetHPSpawner _output_get self)
  (Default|RandomizeHP _output_get))

(fn SpawnHPatSpawnPoint
  (CallFunction|SpawnHP (Transformation|GetWorldLocation (Variables|/Game/InfiniteMatrix/Blueprints/Unneeded/BP_HealthPack.BP_HealthPack_C|GetSpawnHPPoint (Variables|Default|GetNewestHP)))))

(fn SpawnInitialHP
  (for _index (range 0 2)
    (Utilities|IsValid (Variables|Default|GetNewestHP)
      (:Is%20Not%20Valid
        (CallFunction|SpawnHP (Transformation|GetActorLocation (Game|Player|GetPlayerPawn 0)))))))